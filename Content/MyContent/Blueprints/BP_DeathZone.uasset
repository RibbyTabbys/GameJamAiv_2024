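; BP_DeathZone is a trigger actor that ends the game when the player pawn overlaps its DeathZone component.
; On begin overlap, it confirms the player pawn is inside, pauses the game and adds a WBP_GameOver widget to the viewport.
; It then switches input to UI-only and shows the mouse cursor.
; BeginPlay caches the pawn as BP_Player, but the overlap logic does not use that reference.
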(event OnComponentBeginOverlap(DeathZone)
  (params (OverlappedComponent :type Primitive%20Component%20Object%20Reference) (OtherActor :type Actor%20Object%20Reference) (OtherComp :type Primitive%20Component%20Object%20Reference) (OtherBodyIndex :type Integer) (bFromSweep :type Boolean) (SweepResult :type Hit%20Result%20Structure%20%28by%20ref%29))
  (bind _returnvalue (Game|GetPlayerController 0))
  (if (Collision|IsOverlappingActor OverlappedComponent (Game|Player|GetPlayerPawn 0) :!class /Script/Engine.PrimitiveComponent)
    (Game|SetGamePaused true)
    (bind _returnvalue_2 (UserInterface|CreateWidget "/Game/UI_Asset/WBP_GameOver.WBP_GameOver_C"))
    (bind _output_get (Variables|Default|SetWBP_GameOver _returnvalue_2))
    (UserInterface|Viewport|AddtoViewport _output_get 0)
    (Input|SetInputModeUIOnly _returnvalue 0 "DoNotLock" false)
    (Variables|/Script/Engine.PlayerController|SetbShowMouseCursor _returnvalue true)))

(event EventBeginPlay
  (bind _asbp_player (Utilities|Casting|CastToBP_Player (Game|Player|GetPlayerPawn 0)))
  (Variables|Default|SetAs%20BP%20Player _asbp_player))

(fn ConstructionScript)