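; BP_Camera is a rail-style follow camera that becomes player 0's view target on BeginPlay.
; Each Tick it snaps the SpringArm to the point on its Spline closest to the player character.
; The arm's yaw follows the spline direction at that point, with a fixed downward pitch and no roll, so the spline shapes both the camera path and heading.
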(event EventBeginPlay
  (Game|Player|SetViewTargetwithBlend (Game|GetPlayerController 0) self 0.0 "VTBlend_Linear" 0.0 false))

(event Collision|EventActorBeginOverlap
  (params (OtherActor :type Actor%20Object%20Reference)))

(event EventTick
  (params (DeltaSeconds :type Float%20%28single-precision%29))
  (bind _returnvalue (Game|GetPlayerCharacter 0))
  (bind _spline (Variables|Default|GetSpline))
  (bind _springarm (Variables|Default|GetSpringArm))
  (bind _returnvalue_2 (Transformation|GetActorLocation _returnvalue))
  (bind _returnvalue_3 (Spline|FindLocationClosesttoWorldLocation _spline _returnvalue_2 "World"))
  (Transformation|SetWorldLocation _springarm _returnvalue_3 false false)
  (Transformation|SetWorldRotation _springarm (Math|Rotator|MakeRotator 0.0 -25.0 (.yaw (Math|Conversions|RotationFromXVector (Spline|FindDirectionClosesttoWorldLocation (Variables|Default|GetSpline) _returnvalue_3 "World")))) false false))

(fn ConstructionScript)