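; BP_Explosive is an obstacle actor that explodes when it takes damage or receives a qualifying hit.
; Any damage destroys it immediately, while a hit with a downward-facing normal starts a short one-shot timer before destroying it.
; The Destroyed event spawns BP_ExplosionActor at the actor's transform, so every destruction path produces the explosion.
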(event Custom|Explode
  (Actor|DestroyActor))

(event EventBeginPlay)

(event Collision|EventActorBeginOverlap
  (params (OtherActor :type Actor%20Object%20Reference)))

(event EventTick
  (params (DeltaSeconds :type Float%20%28single-precision%29)))

(event Game|Damage|EventAnyDamage
  (params (Damage :type Float%20%28single-precision%29) (DamageType :type Damage%20Type%20Object%20Reference) (InstigatedBy :type Controller%20Object%20Reference) (DamageCauser :type Actor%20Object%20Reference))
  (Actor|DestroyActor))

(event Collision|EventHit
  (params (MyComp :type Primitive%20Component%20Object%20Reference) (Other :type Actor%20Object%20Reference) (OtherComp :type Primitive%20Component%20Object%20Reference) (bSelfMoved :type Boolean) (HitLocation :type Vector :default "0, 0, 0") (HitNormal :type Vector :default "0, 0, 0") (NormalImpulse :type Vector :default "0, 0, 0") (Hit :type Hit%20Result%20Structure%20%28by%20ref%29))
  (if (< (.Z (Class|KismetMathLibrary|BreakVector3f HitNormal)) 0.0)
    (Utilities|Time|SetTimerbyEvent (delegate Custom|Explode) 0.1)))

(event EventDestroyed
  (Game|SpawnActorfromClass "/Game/MyContent/Blueprints/Obstacles/BP_ExplosionActor.BP_ExplosionActor_C" (Transformation|GetActorTransform) "Undefined" 0 0))

(fn ConstructionScript)