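; BP_Helicopter is an obstacle helicopter that flies along a patrol spline.
; On BeginPlay it fetches a BP_HeliPatrol actor from the level and starts a timeline with its play rate set from TimeToComplete.
; Each timeline update maps progress onto spline length and sets the helicopter's transform, using world-space location and local-space rotation from the spline.
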(event Custom|MoveInPatrol
  (bind _splineref (Variables|Default|GetSplineRef))
  (bind _spline (Variables|/Game/MyContent/Blueprints/Obstacles/BP_HeliPatrol.BP_HeliPatrol_C|GetSpline _splineref))
  (Components|Timeline|SetPlayRate (Variables|Default|GetT_MoveInPatrol) (/ 1.0 (Variables|Default|GetTimeToComplete)))
  (bind _moveinpatroltime (Timeline|T_MoveInPatrol Play)
    (:Update
      (Transformation|SetActorTransform (Math|Transform|MakeTransform (Spline|GetLocationatDistanceAlongSpline _spline (Math|Float|Lerp 0.0 (Spline|GetSplineLength (Variables|/Game/MyContent/Blueprints/Obstacles/BP_HeliPatrol.BP_HeliPatrol_C|GetSpline (Variables|Default|GetSplineRef))) _moveinpatroltime) "World") (Spline|GetRotationatDistanceAlongSpline _spline (Math|Float|Lerp 0.0 (Spline|GetSplineLength (Variables|/Game/MyContent/Blueprints/Obstacles/BP_HeliPatrol.BP_HeliPatrol_C|GetSpline (Variables|Default|GetSplineRef))) _moveinpatroltime) "Local") "1.000000,1.000000,1.000000")))))

(event EventBeginPlay
  (bind _returnvalue (Actor|GetActorOfClass "/Game/MyContent/Blueprints/Obstacles/BP_HeliPatrol.BP_HeliPatrol_C"))
  (Variables|Default|SetSplineRef _returnvalue)
  (CallFunction|MoveinPatrol))

(fn ConstructionScript)