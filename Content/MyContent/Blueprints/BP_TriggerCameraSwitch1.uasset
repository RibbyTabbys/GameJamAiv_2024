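; Trigger volume actor that switches the player's view to a wall camera while an actor tagged Player is inside its Box.
; Begin overlap blends player 0's view target to the BP_WallCamera1 actor, and end overlap blends it back to BP_Camera over the same blend time.
; Both cameras are found by class lookup at overlap time rather than by stored references.
; Leftover camera-index cycling logic is present but never runs.
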(event OnComponentBeginOverlap(Box)
  (params (OverlappedComponent :type Primitive%20Component%20Object%20Reference) (OtherActor :type Actor%20Object%20Reference) (OtherComp :type Primitive%20Component%20Object%20Reference) (OtherBodyIndex :type Integer) (bFromSweep :type Boolean) (SweepResult :type Hit%20Result%20Structure%20%28by%20ref%29))
  (if (Actor|ActorHasTag OtherActor "Player")
    (bind _returnvalue (Actor|GetActorOfClass "/Game/MyContent/Blueprints/BP_WallCamera1.BP_WallCamera1_C"))
    (Game|Player|SetViewTargetwithBlend (Game|GetPlayerController 0) _returnvalue 1.0 "VTBlend_Linear" 0.0 false)))

(event OnComponentEndOverlap(Box)
  (params (OverlappedComponent :type Primitive%20Component%20Object%20Reference) (OtherActor :type Actor%20Object%20Reference) (OtherComp :type Primitive%20Component%20Object%20Reference) (OtherBodyIndex :type Integer))
  (if (Actor|ActorHasTag OtherActor "Player")
    (bind _returnvalue (Actor|GetActorOfClass "/Game/MyContent/Blueprints/BP_Camera.BP_Camera_C"))
    (Game|Player|SetViewTargetwithBlend (Game|GetPlayerController 0) _returnvalue 1.0 "VTBlend_Linear" 0.0 false)))

(event EventBeginPlay)

(event Collision|EventActorBeginOverlap
  (params (OtherActor :type Actor%20Object%20Reference)))

(event EventTick
  (params (DeltaSeconds :type Float%20%28single-precision%29)))

(fn ConstructionScript)